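; BP_Net is a fishing net actor that reacts to being hit by the first-person projectile.
; On hit, a timeline eases the Net component down to a smaller scale.
; A half-second delay fired from that timeline's update then hides Net, reveals the FishingNet平面 component and starts a second timeline that tilts PolySurface49.
; Both lerps start from the current transform each update, so the easing compounds.
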(event OnComponentHit(Net)
  (params (HitComponent :type Primitive%20Component%20Object%20Reference) (OtherActor :type Actor%20Object%20Reference) (OtherComp :type Primitive%20Component%20Object%20Reference) (NormalImpulse :type Vector :default "0, 0, 0") (Hit :type Hit%20Result%20Structure%20%28by%20ref%29))
  (Utilities|Casting|CastToBP_FirstPersonProjectile OtherActor)
  (bind _newtrack_0 (Timeline|Timeline Play)
    (:Update
      (Transformation|SetRelativeScale3D (Variables|Default|GetNet) (Math|Vector|Lerp(Vector) (Variables|/Script/Engine.SceneComponent|GetRelativeScale3D (Variables|Default|GetNet)) "0.300000,0.300000,0.300000" _newtrack_0))
      (Utilities|FlowControl|Delay 0.5)
      (Rendering|SetVisibility (Variables|Default|GetNet) false false)
      (Rendering|SetVisibility (Variables|Default|Getfishing_net_平面) true false)
      (bind _newtrack_0_2 (Timeline|Timeline_0 Play)
        (:Update
          (Transformation|SetRelativeRotation (Variables|Default|GetpolySurface49) (Math|Rotator|Lerp(Rotator) (Variables|/Script/Engine.SceneComponent|GetRelativeRotation (Variables|Default|GetpolySurface49)) "0.000000,0.000000,30.000000" _newtrack_0_2) false false))))))

(event EventBeginPlay)

(event Collision|EventActorBeginOverlap
  (params (OtherActor :type Actor%20Object%20Reference)))

(event EventTick
  (params (DeltaSeconds :type Float%20%28single-precision%29)))

(fn ConstructionScript)